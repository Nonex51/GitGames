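; Tank Blueprint that sets up the barrel reference and handles aim-view input.
; On BeginPlay it passes the Barret component to SetBarrelReference.
; The AimAzimuth axis yaws AzimuthGimbal and AimElevation pitches SpringArm in local space, splitting the two rotations across components.
; Both scale input by world delta seconds for frame-rate-independent turning, with no pitch clamp in the graph.
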(event EventBeginPlay
  (Class|Tank|SetBarrelReference (Variables|Default|GetBarret)))

(event Collision|EventActorBeginOverlap
  (params (OtherActor :type Actor%20Object%20Reference)))

(event EventTick
  (params (DeltaSeconds :type Float%20%28single-precision%29)))

(event Input|AxisEvents|InputAxisAimAzimuth
  (params (AxisValue :type Float%20%28single-precision%29))
  ;[1 1 1] Input AimVision
  (Transformation|AddLocalRotation (Variables|Default|GetAzimuth%20Gimbal) (Math|Conversions|RotationFromXVector (Class|KismetMathLibrary|CreateVectorfromYawPitch (* AxisValue (Utilities|Time|GetWorldDeltaSeconds) 1e+02) 0.0 1.0)) false false))

(event Input|AxisEvents|InputAxisAimElevation
  (params (AxisValue :type Float%20%28single-precision%29))
  ;[1 1 1] Input AimVision
  (Transformation|AddLocalRotation (Variables|Default|GetSpringArm) (Math|Conversions|RotationFromXVector (Class|KismetMathLibrary|CreateVectorfromYawPitch 0.0 (* AxisValue (Utilities|Time|GetWorldDeltaSeconds) 1e+02) 1.0)) false false))

(fn ConstructionScript)